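; Exploding car prop for a platformer that blows up on overlap, launching the player character upward after a brief delay.
; A gated overlap fires the explosion effect, layered sounds and a timeline that deforms the mask and roof parts.
; A retriggerable delay reopens the gate and restores rotations saved at construction, though not the roof's offset.
; The close-contact trigger shuts the gate and restarts that delay, blocking explosions meanwhile.
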(event OnComponentBeginOverlap(Closecontacttrigger)
  (params (OverlappedComponent :type Primitive%20Component%20Object%20Reference) (OtherActor :type Actor%20Object%20Reference) (OtherComp :type Primitive%20Component%20Object%20Reference) (OtherBodyIndex :type Integer) (bFromSweep :type Boolean) (SweepResult :type Hit%20Result%20Structure%20%28by%20ref%29))
  (bind _explosion (Variables|ExplodingCarBP|GetExplosion))
  (Utilities|FlowControl|Sequence
    (:then_0
      (Utilities|FlowControl|Gate false) ; enters at Close
    )
    (:then_1
      ;[1 1 1] Reset object
      (Utilities|FlowControl|RetriggerableDelay 1e+01)
      (Transformation|SetWorldRotation (Variables|ExplodingCarBP|GetMask) (Variables|Default|GetMaskRotation) false false)
      (Transformation|SetWorldRotation (Variables|ExplodingCarBP|GetRoofBack) (Variables|Default|GetRoofBackRotation) false false)
      (Transformation|SetWorldRotation (Variables|ExplodingCarBP|GetRoofTop) (Variables|Default|GetRoofMidROtation) false false)
      (Utilities|FlowControl|Gate false) ; enters at Open
    )))

(event OnComponentBeginOverlap(Colission)
  (params (OverlappedComponent :type Primitive%20Component%20Object%20Reference) (OtherActor :type Actor%20Object%20Reference) (OtherComp :type Primitive%20Component%20Object%20Reference) (OtherBodyIndex :type Integer) (bFromSweep :type Boolean) (SweepResult :type Hit%20Result%20Structure%20%28by%20ref%29))
  (bind _explosion (Variables|ExplodingCarBP|GetExplosion))
  (Utilities|FlowControl|Gate false :!label _label
    (:Exit
      (Utilities|FlowControl|Sequence
        (:then_0
          ;[1 1 1] Make some noise
          (Utilities|FlowControl|Sequence
            (:then_0
              ;;[1 1 1] Sound
              (Audio|SpawnSoundAttached "/Game/Sounds/Foley_Physics/Explosions/Explosions_Large_Cue.Explosions_Large_Cue" _explosion "None" "0, 0, 0" "0, 0, 0" "KeepRelativeOffset" false 1.3 1.0))
            (:then_1
              (Components|Activation|Activate (Variables|ExplodingCarBP|GetExplosion) false)
              (Audio|SpawnSoundAttached "/Game/Sounds/Foley_Physics/Explosions/Explosions_Large_Stereo_Cue.Explosions_Large_Stereo_Cue" _explosion "None" "0, 0, 0" "0, 0, 0" "KeepRelativeOffset" false 0.3 1.3)
              ;[1 1 1] Reset object
              (Utilities|FlowControl|RetriggerableDelay 1e+01)
              (Transformation|SetWorldRotation (Variables|ExplodingCarBP|GetMask) (Variables|Default|GetMaskRotation) false false)
              (Transformation|SetWorldRotation (Variables|ExplodingCarBP|GetRoofBack) (Variables|Default|GetRoofBackRotation) false false)
              (Transformation|SetWorldRotation (Variables|ExplodingCarBP|GetRoofTop) (Variables|Default|GetRoofMidROtation) false false)
              (goto _label Open))
            (:then_2
              (bind _angle (Timeline|Timeline_0 PlayFromStart)
                (:Update
                  (Transformation|AddLocalRotation (Variables|ExplodingCarBP|GetMask) (Math|Rotator|MakeRotator 0.0 _angle 0.0) false false)
                  (Transformation|AddLocalRotation (Variables|ExplodingCarBP|GetRoofBack) (Math|Rotator|MakeRotator 0.0 (* _angle -0.12) 0.0) false false)
                  (Transformation|AddLocalOffset (Variables|ExplodingCarBP|GetRoofTop) (Math|Vector|MakeVector 0.0 0.0 (* _angle -0.1)) false false))))))
        (:then_1
          ;[1 1 1] Launch the character
          (Utilities|FlowControl|Delay 0.1)
          (bind _asplatformer_character (Utilities|Casting|CastToPlatformerCharacter (Game|Player|GetPlayerPawn 0)))
          (Character|LaunchCharacter _asplatformer_character (Math|Vector|MakeVector 0.0 0.0 (Variables|Default|GetLaunchSpeed)) false true))
        (:then_2
          (goto _label Close))))))

(event Collision|EventActorBeginOverlap
  (params (OtherActor :type Actor%20Object%20Reference))
  (bind _explosion (Variables|ExplodingCarBP|GetExplosion))
  (Utilities|FlowControl|Gate false :!label _label
    (:Exit
      (Utilities|FlowControl|Sequence
        (:then_0
          ;[1 1 1] Make some noise
          (Utilities|FlowControl|Sequence
            (:then_0
              ;;[1 1 1] Sound
              (Audio|SpawnSoundAttached "/Game/Sounds/Foley_Physics/Explosions/Explosions_Large_Cue.Explosions_Large_Cue" _explosion "None" "0, 0, 0" "0, 0, 0" "KeepRelativeOffset" false 1.3 1.0))
            (:then_1
              (Components|Activation|Activate (Variables|ExplodingCarBP|GetExplosion) false)
              (Audio|SpawnSoundAttached "/Game/Sounds/Foley_Physics/Explosions/Explosions_Large_Stereo_Cue.Explosions_Large_Stereo_Cue" _explosion "None" "0, 0, 0" "0, 0, 0" "KeepRelativeOffset" false 0.3 1.3)
              ;[1 1 1] Reset object
              (Utilities|FlowControl|RetriggerableDelay 1e+01)
              (Transformation|SetWorldRotation (Variables|ExplodingCarBP|GetMask) (Variables|Default|GetMaskRotation) false false)
              (Transformation|SetWorldRotation (Variables|ExplodingCarBP|GetRoofBack) (Variables|Default|GetRoofBackRotation) false false)
              (Transformation|SetWorldRotation (Variables|ExplodingCarBP|GetRoofTop) (Variables|Default|GetRoofMidROtation) false false)
              (goto _label Open))
            (:then_2
              (bind _angle (Timeline|Timeline_0 PlayFromStart)
                (:Update
                  (Transformation|AddLocalRotation (Variables|ExplodingCarBP|GetMask) (Math|Rotator|MakeRotator 0.0 _angle 0.0) false false)
                  (Transformation|AddLocalRotation (Variables|ExplodingCarBP|GetRoofBack) (Math|Rotator|MakeRotator 0.0 (* _angle -0.12) 0.0) false false)
                  (Transformation|AddLocalOffset (Variables|ExplodingCarBP|GetRoofTop) (Math|Vector|MakeVector 0.0 0.0 (* _angle -0.1)) false false))))))
        (:then_1
          ;[1 1 1] Launch the character
          (Utilities|FlowControl|Delay 0.1)
          (bind _asplatformer_character (Utilities|Casting|CastToPlatformerCharacter (Game|Player|GetPlayerPawn 0)))
          (Character|LaunchCharacter _asplatformer_character (Math|Vector|MakeVector 0.0 0.0 (Variables|Default|GetLaunchSpeed)) false true))
        (:then_2
          (goto _label Close))))))

(fn ConstructionScript
  (Variables|Default|SetMaskRotation (Transformation|GetWorldRotation (Variables|ExplodingCarBP|GetMask)))
  (Variables|Default|SetRoofBackRotation (Transformation|GetWorldRotation (Variables|ExplodingCarBP|GetRoofBack)))
  (Variables|Default|SetRoofMidROtation (Transformation|GetWorldRotation (Variables|ExplodingCarBP|GetRoofTop))))